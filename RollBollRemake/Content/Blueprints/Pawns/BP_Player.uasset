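; BP_Player is the player pawn for an obstacle-avoidance runner with constant forward motion.
; While movement is enabled, Tick sweeps it forward along X, applies clamped horizontal input on Y and spins Scene1.
; Hitting a BP_Obstacle destroys the pawn, while HandleGameOver stops movement, disables input and switches widgets through BP_WidgetsManager.
; HandleSpeed raises forward speed at score intervals until it passes a cap.
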(event EventTick
  (params (DeltaSeconds :type Float%20%28single-precision%29))
  (bind _returnvalue (Transformation|GetActorLocation))
  (if (Variables|Default|GetbMovement)
    (Transformation|SetActorLocation (Math|Vector|MakeVector (+ (Variables|Default|GetSpeed) (.x _returnvalue)) (Math|Float|Clamp(Float) (+ (.y _returnvalue) (* (Input|AxisValues|GetHorizontal) (Variables|Default|GetHorizontalSpeed))) -1.8e+02 1.8e+02) (.z _returnvalue)) true false)
    (Transformation|AddLocalRotation (Variables|Default|GetScene1) (Math|Rotator|MakeRotator 0.0 (Variables|Default|GetRotationSpeed) 0.0) false false)))

(fn ConstructionScript)

(fn OnObstacleHit
  (params (OtherActor :type Actor%20Object%20Reference))
  (Utilities|Casting|CastToBP_Obstacle OtherActor)
  (Actor|DestroyActor))

(fn HandleGameOver
  (Input|DisableInput (Game|GetPlayerController 0))
  (Variables|Default|SetbMovement false)
  (bind _returnvalue (Actor|GetActorOfClass "/Game/Blueprints/BP_WidgetsManager.BP_WidgetsManager_C"))
  (Default|RemoveWidgetGameplay _returnvalue)
  (Default|SetCurrentWidgettoGameOver _returnvalue))

(fn StartGame
  (Variables|Default|SetbMovement true))

(fn HandleSpeed
  (if (== (Math|Integer|%(Integer) (Variables|/Game/Blueprints/BP_ScoreComponent.BP_ScoreComponent_C|GetScore (Variables|Default|GetBP_ScoreComponent)) (Variables|Default|GetIncreaseSpeedPerObstacle)) 0)
    (if (<= (Variables|Default|GetSpeed) 1.8e+02)
      (Variables|Default|SetSpeed (+ (Variables|Default|GetSpeed) (Variables|Default|GetSpeedIncrease)))
      (Development|PrintString (Utilities|String|ToString(Float) (Variables|Default|GetSpeed))))))