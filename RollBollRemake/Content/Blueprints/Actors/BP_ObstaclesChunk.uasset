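; BP_ObstaclesChunk is an actor that lays out a short run of obstacles when play begins.
; On BeginPlay it spawns three BP_Obstacle actors at evenly spaced steps along world X from its own location, starting at its origin and separated by DistanceBetweenObstacles.
; Each obstacle keeps the chunk's Y but is placed at world Z zero.
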(event EventBeginPlay
  (CallFunction|SpawnObstacle 0.0)
  (CallFunction|SpawnObstacle (Variables|Default|GetDistanceBetweenObstacles))
  (CallFunction|SpawnObstacle (* 2 (Variables|Default|GetDistanceBetweenObstacles))))

(fn ConstructionScript)

(fn SpawnObstacle
  (params (Distance :type Float%20%28single-precision%29))
  (bind _returnvalue (Transformation|GetActorLocation))
  (Game|SpawnActorfromClass "/Game/Blueprints/Actors/BP_Obstacle.BP_Obstacle_C" (Math|Transform|MakeTransform (Math|Vector|MakeVector (+ Distance (.x _returnvalue)) (.y _returnvalue) 0.0)) "Undefined" 0 0))